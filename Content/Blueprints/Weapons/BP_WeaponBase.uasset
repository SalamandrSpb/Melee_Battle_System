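; Base weapon Blueprint that detects hits on BP_AIEnemy actors and changes their health.
; TraceWeapon plays a timeline that, on each update, sphere-traces the Visibility channel between two point components on the weapon, with debug drawing enabled.
; An enemy hit calls ChangeHealth with a fixed amount for the neck bone or the Damage variable otherwise, then StopTrace halts the timeline.
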(event Custom|TraceWeapon
  (Timeline|TimeTrace Play
    (:Update
      (bind (_outhit _returnvalue) (Collision|SphereTraceByChannel (Transformation|GetWorldLocation (Variables|Default|GetPointTrace)) (Transformation|GetWorldLocation (Variables|Default|GetPointTrace2)) 0.0 "TraceTypeQuery1" false 0 "ForDuration"))
      (if _returnvalue
        (bind _asbp_aienemy (Utilities|Casting|CastToBP_AIEnemy (.HitActor (Collision|BreakHitResult _outhit))))
        (if (Utilities|Name|Equal(Name) (.HitBoneName (Collision|BreakHitResult _outhit)) "neck_01")
          (Default|ChangeHealth _asbp_aienemy 2e+01)
          (CallFunction|StopTrace)
          (else
            (Default|ChangeHealth _asbp_aienemy (Variables|Default|GetDamage))
            (CallFunction|StopTrace)))))))

(event Custom|StopTrace
  (Timeline|TimeTrace Stop
    (:Update
      (bind (_outhit _returnvalue) (Collision|SphereTraceByChannel (Transformation|GetWorldLocation (Variables|Default|GetPointTrace)) (Transformation|GetWorldLocation (Variables|Default|GetPointTrace2)) 0.0 "TraceTypeQuery1" false 0 "ForDuration"))
      (if _returnvalue
        (bind _asbp_aienemy (Utilities|Casting|CastToBP_AIEnemy (.HitActor (Collision|BreakHitResult _outhit))))
        (if (Utilities|Name|Equal(Name) (.HitBoneName (Collision|BreakHitResult _outhit)) "neck_01")
          (Default|ChangeHealth _asbp_aienemy 2e+01)
          (CallFunction|StopTrace)
          (else
            (Default|ChangeHealth _asbp_aienemy (Variables|Default|GetDamage))
            (CallFunction|StopTrace)))))))

(event EventBeginPlay)

(event Collision|EventActorBeginOverlap
  (params (OtherActor :type Actor%20Object%20Reference)))

(event EventTick
  (params (DeltaSeconds :type Float%20%28single-precision%29)))

(fn ConstructionScript)