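; Player character Blueprint for melee combat, handling movement, camera look, toggled sprint, arming, blocking and directional attacks.
; On BeginPlay it spawns a sword and shield on mesh sockets; arming moves the sword between hand and sheath, with delayed sheathing.
; Attacks require being armed and not blocking; DirAttack turns movement input into a direction that selects a montage from AttackAnim.
; Montage notifies start and stop the weapon's hit trace.
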(event EventBeginPlay
  (bind _returnvalue (Game|SpawnActorfromClass "/Game/Blueprints/Weapons/BP_Sword.BP_Sword_C" (Transformation|GetActorTransform) "Undefined" 0 0))
  (bind _output_get (Variables|Default|SetWeapon _returnvalue))
  (Transformation|AttachComponentToComponent _output_get (Variables|Default|GetSkeletalMesh) (Variables|Default|GetSheathSocket) "SnapToTarget" "SnapToTarget" "SnapToTarget" true)
  (bind _returnvalue_2 (Game|SpawnActorfromClass "/Game/Blueprints/Weapons/BP_Shield.BP_Shield_C" (Transformation|GetActorTransform) "Undefined" 0 0))
  (Transformation|AttachComponentToComponent _returnvalue_2 (Variables|Default|GetSkeletalMesh) (Variables|/Game/Blueprints/Weapons/BP_WeaponBase.BP_WeaponBase_C|GetSocketName _returnvalue_2) "SnapToTarget" "SnapToTarget" "SnapToTarget" true))

(event Collision|EventActorBeginOverlap
  (params (OtherActor :type Actor%20Object%20Reference)))

(event EventTick
  (params (DeltaSeconds :type Float%20%28single-precision%29)))

(event Input|ActionEvents|InputActionArmed
  (params (Key :type Key%20Structure :default "None"))
  (bind _weapon (Variables|Default|GetWeapon))
  ;[1 1 1] Вооружение
  (:Pressed
    (if (not (Variables|Default|GetIsBlock))
      (bind _output_get (Variables|Default|SetIsArmed (not (Variables|Default|GetIsArmed))))
      (if _output_get
        (Transformation|AttachComponentToComponent _weapon (Variables|Default|GetSkeletalMesh) (Variables|/Game/Blueprints/Weapons/BP_WeaponBase.BP_WeaponBase_C|GetSocketName _weapon) "SnapToTarget" "SnapToTarget" "SnapToTarget" true)
        (else
          (Utilities|FlowControl|Delay 1.1)
          (Transformation|AttachComponentToComponent (Variables|Default|GetWeapon) (Variables|Default|GetSkeletalMesh) (Variables|Default|GetSheathSocket) "SnapToTarget" "SnapToTarget" "SnapToTarget" true))))))

(event Input|ActionEvents|InputActionSprint
  (params (Key :type Key%20Structure :default "None"))
  ;[1 1 1] Спринт
  (:Pressed
    (bind _output_get (Variables|Default|SetIsSprint (not (Variables|Default|GetIsSprint))))
    (if _output_get
      (Variables|/Script/Engine.CharacterMovementComponent|SetMaxWalkSpeed (Variables|Character|GetCharacterMovement) (Variables|Default|GetSprintSpeed))
      (else
        (Variables|/Script/Engine.CharacterMovementComponent|SetMaxWalkSpeed (Variables|Character|GetCharacterMovement) (Variables|Default|GetDefaultSpeed))))))

(event Input|ActionEvents|InputActionAttack
  (params (Key :type Key%20Structure :default "None"))
  (bind _weapon (Variables|Default|GetWeapon))
  (:Pressed
    (Variables|Default|SetIsAttack (not (Variables|Default|GetIsAttack)))
    ;[1 1 1] Анимация атаки в зависимости от направления
    (if (and (Variables|Default|GetIsArmed) (not (Variables|Default|GetIsBlock)))
      (CallFunction|DirAttack)
      (Animation|Montage|PlayMontage (Variables|Default|GetSkeletalMesh) (.Value (Utilities|Map|Find (Variables|Default|GetAttackAnim) (Variables|Default|GetDirectionAttack)))
        (:OnNotifyBegin
          (Default|TraceWeapon _weapon))
        (:OnNotifyEnd
          (Default|StopTrace _weapon)))))
  (:Released
    (Variables|Default|SetIsAttack (not (Variables|Default|GetIsAttack)))))

(event Input|ActionEvents|InputActionBlock
  (params (Key :type Key%20Structure :default "None"))
  (:Pressed
    (Variables|Default|SetIsBlock (not (Variables|Default|GetIsBlock))))
  (:Released
    (Variables|Default|SetIsBlock (not (Variables|Default|GetIsBlock)))))

(event Input|AxisEvents|InputAxisMoveFoward
  (params (AxisValue :type Float%20%28single-precision%29))
  ;[1 1 1] Передвижение
  (bind _output_get (Variables|Default|SetDirectionX AxisValue))
  (Pawn|Input|AddMovementInput (Transformation|GetActorForwardVector) _output_get false))

(event Input|AxisEvents|InputAxisMoveRight
  (params (AxisValue :type Float%20%28single-precision%29))
  ;[1 1 1] Передвижение
  (bind _output_get (Variables|Default|SetDirectionY AxisValue))
  (Pawn|Input|AddMovementInput (Transformation|GetActorRightVector) _output_get false))

(event Input|AxisEvents|InputAxisLookUp
  (params (AxisValue :type Float%20%28single-precision%29))
  ;[1 1 1] Camera
  (Pawn|Input|AddControllerPitchInput AxisValue))

(event Input|AxisEvents|InputAxisTurnAround
  (params (AxisValue :type Float%20%28single-precision%29))
  ;[1 1 1] Camera
  (Pawn|Input|AddControllerYawInput AxisValue))

(fn ConstructionScript)

(fn DirAttack
  (if (!= (Variables|Default|GetDirectionX) 0.0)
    (if (> (Variables|Default|GetDirectionX) 0.0)
      (Variables|Default|SetDirectionAttack "NewEnumerator0")
      (else
        (Variables|Default|SetDirectionAttack "NewEnumerator1")))
    (elif (> (Variables|Default|GetDirectionY) 0.0)
      (Variables|Default|SetDirectionAttack "NewEnumerator3")
      (else
        (Variables|Default|SetDirectionAttack "NewEnumerator2")))))