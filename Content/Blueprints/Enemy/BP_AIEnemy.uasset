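; BP_AIEnemy is an enemy actor with a health value shown on a text render component.
; The health text is set on BeginPlay and refreshed whenever the ChangeHealth event subtracts damage.
; At zero or below, the mesh switches to physics simulation as a ragdoll-style death and the capsule ignores WorldStatic collision.
; The file holds no AI logic, and its Tick and overlap events are empty.
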(event Custom|ChangeHealth
  (params (Damage :type Float%20%28single-precision%29))
  (bind _output_get (Variables|Default|SetHealth (- (Variables|Default|GetHealth) Damage)))
  (Rendering|Components|TextRender|SetText (Variables|Default|GetHealthRender) (Utilities|Text|ToText(Float) _output_get "HalfToEven"))
  (if (<= (Variables|Default|GetHealth) 0.0)
    (Collision|SetCollisionEnabled (Variables|Character|GetMesh) "QueryAndPhysics")
    (Physics|SetSimulatePhysics (Variables|Character|GetMesh) true)
    (Collision|SetCollisionResponsetoChannel (Variables|Collision|GetCapsuleComponent) "ECC_WorldStatic" "ECR_Ignore")))

(event EventBeginPlay
  (Rendering|Components|TextRender|SetText (Variables|Default|GetHealthRender) (Utilities|Text|ToText(Float) (Variables|Default|GetHealth) "HalfToEven")))

(event Collision|EventActorBeginOverlap
  (params (OtherActor :type Actor%20Object%20Reference)))

(event EventTick
  (params (DeltaSeconds :type Float%20%28single-precision%29)))

(fn ConstructionScript)